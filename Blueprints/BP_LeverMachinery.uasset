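; BP_LeverMachinery is a puzzle lever that needs a BP_Sword as its missing piece before it can lower TriggeredActor.
; Interacting with the sword attached consumes it and shows StaticMesh1; empty-handed interactions toggle a hint dialogue that locks input.
; Later interactions play the Move timeline, offsetting the target downward from its current location each update.
; On finish it saves its display name to the GameInstance as solved, blocking replays.
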(event EventBeginPlay
  (|CallParentFunction))

(event Collision|EventActorBeginOverlap
  (params (OtherActor :type Actor%20Object%20Reference))
  (|CallParentFunction OtherActor)
  (Collision|SetCollisionEnabled (Variables|Default|GetStaticMesh1) "NoCollision"))

(event EventTick
  (params (DeltaSeconds :type Float%20%28single-precision%29))
  (|CallParentFunction DeltaSeconds) ; This node is disabled and will not be called.\nDrag off pins to build functionality.
)

(event EventInteraction
  (bind _returnvalue (Game|GetPlayerController 0))
  (bind _returnvalue_2 (Game|GetPlayerController 0))
  (bind _triggeredactor (Variables|Default|GetTriggeredActor))
  (bind _staticmesh1 (Variables|Default|GetStaticMesh1))
  (bind _returnvalue_3 (Transformation|GetActorLocation _triggeredactor))
  (if (Variables|Default|GetwasTriggered)
    (bind _solvedactors (Class|IGet|GetSolvedActors(Message) (Game|GetGameInstance)))
    (if (not (Utilities|Array|ContainsItem _solvedactors (Utilities|GetDisplayName self)))
      (bind _newtrack_0 (Timeline|Move Play)
        (:Update
          (Transformation|SetActorLocation (Variables|Default|GetTriggeredActor) (Math|Vector|Lerp(Vector) _returnvalue_3 (- _returnvalue_3 "0.000000,0.000000,10.000000") _newtrack_0) false false))
        (:Finished
          (Class|ISave|SaveSolvedActor(Message) (Game|GetGameInstance) (Utilities|GetDisplayName self)))))
    (else
      (bind _actor (Class|IGet|GetAttachedActorLocal(Message) (Game|GetGameInstance)))
      (if (Utilities|IsValid _actor)
        (if (== (Utilities|GetClass _actor) "/Game/Custom/Blueprints/Blueprints/BP_Sword.BP_Sword_C")
          (Variables|Default|SetwasTriggered true)
          (Class|IDestroy|DestroyAttachedActor(Message) (Game|Player|GetPlayerPawn 0) true)
          (Rendering|SetVisibility _staticmesh1 true false)
          (Collision|SetCollisionEnabled _staticmesh1 "QueryAndPhysics")
          (Variables|Default|SetwasTriggered true))
        (else
          (Utilities|FlowControl|FlipFlop
            (:A
              (bind _returnvalue_4 (UserInterface|CreateWidget "/Game/Custom/Blueprints/Widgets/WB_Dialogue.WB_Dialogue_C" (Game|GetPlayerController 0)))
              (bind _output_get (Variables|Default|SetDialogueBox _returnvalue_4))
              (Variables|/Script/UMG.TextBlock|SetText (Variables|/Game/Custom/Blueprints/Widgets/WB_Dialogue.WB_Dialogue_C|GetDialogue1 _output_get) "Seems like it is missing a piece")
              (UserInterface|Viewport|AddtoViewport _output_get 0)
              (Input|SetIgnoreLookInput _returnvalue_2 true)
              (Input|SetIgnoreMoveInput _returnvalue_2 true)
              (Class|ISave|SaveinWidget(Message) _returnvalue_2 true))
            (:B
              (Widget|RemovefromParent (Variables|Default|GetDialogueBox))
              (Input|SetIgnoreLookInput _returnvalue false)
              (Input|SetIgnoreMoveInput _returnvalue false)
              (Class|ISave|SaveinWidget(Message) _returnvalue false))))))))

(fn ConstructionScript
  (|CallParentFunction))