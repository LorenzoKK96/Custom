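; Secret library door puzzle actor that accepts a BP_Tome and slides along Y once solved.
; Interaction snaps the player's carried tome onto it and compares its name to CorrectBook, recording a match in the GameInstance.
; An incorrect tome stays until the next interaction pushes it back out.
; BeginPlay calls Resolve when the solved-puzzle string contains "Library", running the Rotating timeline, which offsets from the current location each update.
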(event EventBeginPlay
  (|CallParentFunction)
  (bind _solvedpuzzles (Class|IGet|GetSolvedPuzzle(Message) (Game|GetGameInstance)))
  (if (Utilities|Set|Contains _solvedpuzzles "Library")
    (CallFunction|Resolve)))

(event Collision|EventActorBeginOverlap
  (params (OtherActor :type Actor%20Object%20Reference))
  (|CallParentFunction OtherActor) ; This node is disabled and will not be called.\nDrag off pins to build functionality.
)

(event EventTick
  (params (DeltaSeconds :type Float%20%28single-precision%29))
  (|CallParentFunction DeltaSeconds))

(event EventResolve
  (bind _returnvalue (Transformation|GetActorLocation))
  (bind _rotate (Timeline|Rotating Play)
    (:Update
      (Transformation|SetActorLocation (Math|Vector|Lerp(Vector) _returnvalue (+ _returnvalue (Math|Vector|MakeVector 0.0 (Variables|Default|GetMovement) 0.0)) _rotate) false false))))

(event EventInteraction
  (bind _returnvalue (Game|GetGameInstance))
  (bind _returnvalue_2 (Transformation|GetActorLocation))
  (bind _returnvalue_3 (Game|GetGameInstance))
  (bind _self self)
  (bind _self_2 self)
  (bind _returnvalue_4 (Utilities|GetDisplayName _self))
  (bind _returnvalue_5 (Transformation|GetActorRotation _self_2))
  (if (not (Variables|Default|Getsolved))
    (if (Utilities|IsValid (Variables|Default|GetreferenceActor))
      (Class|IControlAttach|Detach(Message) (Variables|Default|GetreferenceActor))
      (Transformation|SetActorLocation (Variables|Default|GetreferenceActor) (Math|Vector|MakeVector (- (.x _returnvalue_2) (Variables|Default|GetPushTomeX)) (.y _returnvalue_2) (+ (.z _returnvalue_2) (Variables|Default|GetPushTomeZ))) false false)
      (Collision|SetActorEnableCollision true)
      (Variables|Default|SetreferenceActor 0)
      (else
        (bind _actor (Class|IGet|GetAttachedActorLocal(Message) _returnvalue_3))
        (if (and (Utilities|IsValid _actor) (== (Utilities|GetClass _actor) "/Game/Custom/Blueprints/Blueprints/BP_Tome.BP_Tome_C"))
          (bind _output_get (Variables|Default|SetreferenceActor _actor))
          (Class|IControlAttach|Detach(Message) _output_get)
          (Class|ISave|SaveAttachedActorLocal(Message) _returnvalue_3)
          (Transformation|AttachActorToActor (Variables|Default|GetreferenceActor) self "None" "SnapToTarget" "SnapToTarget" "KeepWorld" true)
          (Transformation|AddActorLocalOffset (Variables|Default|GetreferenceActor) "25.000000,175.000000,120.000000" false false)
          (Transformation|SetActorRotation (Variables|Default|GetreferenceActor) (Math|Rotator|MakeRotator (.roll _returnvalue_5) (+ (.pitch _returnvalue_5) 9e+01) (.yaw _returnvalue_5)))
          (bind _attachedname (Class|IGet|GetAttachedActorName(Message) (Game|GetGameInstance)))
          (if (Utilities|Enum|Equal(Enum) _attachedname (Variables|Default|GetcorrectBook))
            (Development|PrintString "CorrectBook")
            (Collision|SetActorEnableCollision (Variables|Default|GetreferenceActor) false)
            (Class|IDestroy|DestroyAttachedActor(Message) (Game|Player|GetPlayerPawn 0))
            (Class|ISave|SaveSolvedActorRef(Message) _returnvalue _self _returnvalue_4)
            (Class|ISave|SaveSolvedActor(Message) _returnvalue _returnvalue_4)
            (Variables|Default|SetSolved true)
            (else
              (Development|PrintString "Incorrect")
              (Collision|SetActorEnableCollision (Variables|Default|GetreferenceActor) false)
              (Class|IDestroy|DestroyAttachedActor(Message) (Game|Player|GetPlayerPawn 0)))))))))

(fn ConstructionScript
  (|CallParentFunction))