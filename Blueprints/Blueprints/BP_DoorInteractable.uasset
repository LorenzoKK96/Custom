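; Interactable door that swings open once "ChurchKey" is in the GameInstance's solved-actor list and the player interacts inside RightTrigger.
; A Timeline rotates the door, then saves its display name as solved and destroys the player's attached actor; BeginPlay uses that record to restore the open state.
; Without the key, interacting in WrongTrigger can toggle a dialogue widget via FlipFlop, locking look and move input while shown.
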(event OnComponentBeginOverlap(RightTrigger)
  (params (OverlappedComponent :type Primitive%20Component%20Object%20Reference) (OtherActor :type Actor%20Object%20Reference) (OtherComp :type Primitive%20Component%20Object%20Reference) (OtherBodyIndex :type Integer) (bFromSweep :type Boolean) (SweepResult :type Hit%20Result%20Structure%20%28by%20ref%29))
  (if (Components|ComponentHasTag OtherComp "MainBody")
    (Variables|Default|SetisOverlappedGood true)))

(event OnComponentBeginOverlap(WrongTrigger)
  (params (OverlappedComponent :type Primitive%20Component%20Object%20Reference) (OtherActor :type Actor%20Object%20Reference) (OtherComp :type Primitive%20Component%20Object%20Reference) (OtherBodyIndex :type Integer) (bFromSweep :type Boolean) (SweepResult :type Hit%20Result%20Structure%20%28by%20ref%29))
  (if (Components|ComponentHasTag OtherComp "MainBody")
    (Variables|Default|SetisOverlappedWrong true)))

(event OnComponentEndOverlap(RightTrigger)
  (params (OverlappedComponent :type Primitive%20Component%20Object%20Reference) (OtherActor :type Actor%20Object%20Reference) (OtherComp :type Primitive%20Component%20Object%20Reference) (OtherBodyIndex :type Integer))
  (if (Components|ComponentHasTag OtherComp "MainBody")
    (Variables|Default|SetisOverlappedGood false)))

(event OnComponentEndOverlap(WrongTrigger)
  (params (OverlappedComponent :type Primitive%20Component%20Object%20Reference) (OtherActor :type Actor%20Object%20Reference) (OtherComp :type Primitive%20Component%20Object%20Reference) (OtherBodyIndex :type Integer))
  (if (Components|ComponentHasTag OtherComp "MainBody")
    (Variables|Default|SetisOverlappedWrong false)))

(event EventBeginPlay
  (|CallParentFunction)
  (bind _solvedactors (Class|IGet|GetSolvedActors(Message) (Game|GetGameInstance)))
  (if (Utilities|Array|ContainsItem _solvedactors (Utilities|GetDisplayName self))
    (Transformation|SetRelativeRotation (Variables|Default|GetDoor) (Math|Rotator|MakeRotator 0.0 0.0 9e+01) false false)))

(event EventTick
  (params (DeltaSeconds :type Float%20%28single-precision%29))
  (|CallParentFunction DeltaSeconds) ; This node is disabled and will not be called.\nDrag off pins to build functionality.
)

(event EventInteraction
  (bind _returnvalue (Game|GetPlayerController 0))
  (bind _returnvalue_2 (Game|GetPlayerController 0))
  (bind _returnvalue_3 (Game|GetGameInstance))
  (bind _solvedactors (Class|IGet|GetSolvedActors(Message) _returnvalue_3))
  (bind _attachedactor (Class|IGet|GetAttachedActor(Message) _returnvalue_3))
  (if (Utilities|Array|ContainsItem _solvedactors "ChurchKey")
    (if (Variables|Default|GetisOverlappedGood)
      (bind _doorfloat (Timeline|Timeline Play)
        (:Update
          (Transformation|SetRelativeRotation (Variables|Default|GetDoor) (Math|Rotator|MakeRotator 0.0 0.0 (Math|Float|Lerp 0.0 9e+01 _doorfloat)) false false))
        (:Finished
          (Class|ISave|SaveSolvedActor(Message) (Game|GetGameInstance) (Utilities|GetDisplayName self))
          (Class|IDestroy|DestroyAttachedActor(Message) (Game|Player|GetPlayerPawn 0)))))
    (elif (not (Utilities|Array|ContainsItem _solvedactors (Utilities|GetDisplayName self)))
      (if (== _attachedactor 0)
        (if (not (Variables|Default|GetisOverlappedGood))
          (if (Variables|Default|GetisOverlappedWrong) :!label _label
            (Utilities|FlowControl|FlipFlop
              (:A
                (bind _returnvalue_4 (UserInterface|CreateWidget "/Game/Custom/Blueprints/Widgets/WB_Dialogue.WB_Dialogue_C" (Game|GetPlayerController 0)))
                (bind _output_get (Variables|Default|SetDialogueBox _returnvalue_4))
                (UserInterface|Viewport|AddtoViewport _output_get 0)
                (Variables|/Script/UMG.TextBlock|SetText (Variables|/Game/Custom/Blueprints/Widgets/WB_Dialogue.WB_Dialogue_C|GetDialogue1 (Variables|Default|GetDialogueBox)) (Variables|Default|GetText1))
                (Input|SetIgnoreLookInput _returnvalue_2 true)
                (Input|SetIgnoreMoveInput _returnvalue_2 true))
              (:B
                (Widget|RemovefromParent (Variables|Default|GetDialogueBox))
                (Input|SetIgnoreLookInput _returnvalue false)
                (Input|SetIgnoreMoveInput _returnvalue false)))))
        (else
          (goto _label))))))

(fn ConstructionScript
  (|CallParentFunction))