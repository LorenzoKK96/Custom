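; BP_Library is a book-placement puzzle slot that takes a BP_Tome and is solved by the correct book.
; On interaction, it takes the attached tome from the Game Instance, snaps it to itself and clears the player's attached actor.
; A name matching CorrectBook locks the slot and saves it as solved in the Game Instance.
; Otherwise the tome stays until the next interaction pushes it out.
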(event EventBeginPlay
  (|CallParentFunction))

(event Collision|EventActorBeginOverlap
  (params (OtherActor :type Actor%20Object%20Reference))
  (|CallParentFunction OtherActor) ; This node is disabled and will not be called.\nDrag off pins to build functionality.
)

(event EventTick
  (params (DeltaSeconds :type Float%20%28single-precision%29))
  (|CallParentFunction DeltaSeconds) ; This node is disabled and will not be called.\nDrag off pins to build functionality.
)

(event EventInteraction
  (bind _returnvalue (Transformation|GetActorLocation))
  (bind _returnvalue_2 (Game|GetGameInstance))
  (bind _self self)
  (bind _returnvalue_3 (Transformation|GetActorRotation _self))
  (if (not (Variables|Default|Getsolved))
    (if (Utilities|IsValid (Variables|Default|GetreferenceActor))
      (Class|IControlAttach|Detach(Message) (Variables|Default|GetreferenceActor))
      (Transformation|SetActorLocation (Variables|Default|GetreferenceActor) (Math|Vector|MakeVector (- (.x _returnvalue) (Variables|Default|GetPushTomeX)) (.y _returnvalue) (+ (.z _returnvalue) (Variables|Default|GetPushTomeZ))) false false)
      (Collision|SetActorEnableCollision true)
      (Variables|Default|SetreferenceActor 0)
      (else
        (bind _actor (Class|IGet|GetAttachedActorLocal(Message) _returnvalue_2))
        (if (and (Utilities|IsValid _actor) (== (Utilities|GetClass _actor) "/Game/Custom/Blueprints/Blueprints/BP_Tome.BP_Tome_C"))
          (bind _output_get (Variables|Default|SetreferenceActor _actor))
          (Class|IControlAttach|Detach(Message) _output_get)
          (Class|ISave|SaveAttachedActorLocal(Message) _returnvalue_2)
          (Transformation|AttachActorToActor (Variables|Default|GetreferenceActor) self "None" "SnapToTarget" "KeepWorld" "KeepWorld" true)
          (Transformation|AddActorLocalOffset (Variables|Default|GetreferenceActor) "10.000000,0.000000,30.000000" false false)
          (Transformation|SetActorRotation (Variables|Default|GetreferenceActor) (Math|Rotator|MakeRotator (.roll _returnvalue_3) (+ (.pitch _returnvalue_3) 9e+01) (.yaw _returnvalue_3)))
          (bind _attachedname (Class|IGet|GetAttachedActorName(Message) (Game|GetGameInstance)))
          (if (Utilities|Enum|Equal(Enum) _attachedname (Variables|Default|GetcorrectBook))
            (Development|PrintString "CorrectBook")
            (Collision|SetActorEnableCollision (Variables|Default|GetreferenceActor) false)
            (Class|IDestroy|DestroyAttachedActor(Message) (Game|Player|GetPlayerPawn 0))
            (Class|ISave|SaveSolvedActor(Message) (Game|GetGameInstance) (Utilities|GetDisplayName self))
            (Variables|Default|Setsolved true)
            (else
              (Development|PrintString "Incorrect")
              (Collision|SetActorEnableCollision (Variables|Default|GetreferenceActor) false)
              (Class|IDestroy|DestroyAttachedActor(Message) (Game|Player|GetPlayerPawn 0)))))))))

(fn ConstructionScript
  (|CallParentFunction))