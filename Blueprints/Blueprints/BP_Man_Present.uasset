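; BP_Man_Present is an interactable actor, apparently an NPC, that shows a two-part dialogue when the player interacts with it.
; Interaction alternates through a FlipFlop between creating a WB_Dialogue widget filled with Dialog1 and Dialog2, and removing it.
; While the dialogue is open, it ignores the player's look and move input and passes the in-widget state to the pawn via a SaveInWidget message.
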(event EventBeginPlay
  (|CallParentFunction) ; This node is disabled and will not be called.\nDrag off pins to build functionality.
)

(event Collision|EventActorBeginOverlap
  (params (OtherActor :type Actor%20Object%20Reference))
  (|CallParentFunction OtherActor) ; This node is disabled and will not be called.\nDrag off pins to build functionality.
)

(event EventTick
  (params (DeltaSeconds :type Float%20%28single-precision%29))
  (|CallParentFunction DeltaSeconds) ; This node is disabled and will not be called.\nDrag off pins to build functionality.
)

(event EventInteraction
  (bind _returnvalue (Game|Player|GetPlayerPawn 0))
  (bind _returnvalue_2 (Game|GetPlayerController 0))
  (bind _returnvalue_3 (Game|GetPlayerController 0))
  (Utilities|FlowControl|FlipFlop
    (:A
      (bind _returnvalue_4 (UserInterface|CreateWidget "/Game/Custom/Blueprints/Widgets/WB_Dialogue.WB_Dialogue_C" (Game|GetPlayerController 0)))
      (bind _output_get (Variables|Default|SetDialogBox _returnvalue_4))
      (UserInterface|Viewport|AddtoViewport _output_get 0)
      (Variables|/Script/UMG.TextBlock|SetText (Variables|/Game/Custom/Blueprints/Widgets/WB_Dialogue.WB_Dialogue_C|GetDialogue1 (Variables|Default|GetDialogBox)) (Variables|Default|GetDialog1))
      (Variables|/Script/UMG.TextBlock|SetText (Variables|/Game/Custom/Blueprints/Widgets/WB_Dialogue.WB_Dialogue_C|GetDialogue2 (Variables|Default|GetDialogBox)) (Variables|Default|GetDialog2))
      (Input|SetIgnoreLookInput _returnvalue_3 true)
      (Input|SetIgnoreMoveInput _returnvalue_3 true)
      (Class|ISave|SaveinWidget(Message) _returnvalue true))
    (:B
      (Widget|RemovefromParent (Variables|Default|GetDialogBox))
      (Input|SetIgnoreLookInput _returnvalue_2 false)
      (Input|SetIgnoreMoveInput _returnvalue_2 false)
      (Class|ISave|SaveinWidget(Message) _returnvalue false))))

(fn ConstructionScript
  (|CallParentFunction))