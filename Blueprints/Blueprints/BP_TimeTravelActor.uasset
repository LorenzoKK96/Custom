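; Actor that can be held in the player's hand and restores its saved position and held state from the Game Instance, apparently for time travel.
; On BeginPlay it matches its class and display name against saved data, moves its mesh there and removes the entry.
; If flagged as attached, it re-attaches to the player pawn's hand socket.
; Attach disables collision; Detach restores collision and enables mesh physics.
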(event EventIsAttachedInput
  (params (isAttachedInput :type Boolean))
  (Variables|Default|SetisAttached isAttachedInput))

(event Collision|EventActorBeginOverlap
  (params (OtherActor :type Actor%20Object%20Reference)))

(event EventDetach
  (Transformation|DetachFromActor (Variables|Default|GetattachedTo) "KeepWorld" "KeepWorld" "KeepWorld")
  (Physics|SetSimulatePhysics (Variables|Default|GetStaticMesh) true)
  (Collision|SetActorEnableCollision self true)
  (Variables|Default|SetisAttached false))

(event EventAttach
  (params (Owner :type Actor%20Object%20Reference))
  (bind _output_get (Variables|Default|SetattachedTo Owner))
  (Transformation|AttachActorToActor _output_get "hand_rSocket" "SnapToTarget" "SnapToTarget" "KeepRelative" true)
  (Transformation|AddActorLocalOffset (Math|Vector|MakeVector 0.0 0.0 0.0) false false)
  (Collision|SetActorEnableCollision self false)
  (Variables|Default|SetisAttached true))

(event EventBeginPlay
  (bind _returnvalue (Game|GetGameInstance))
  (bind _returnvalue_2 (Game|GetGameInstance))
  (bind _self self)
  ;[1 1 1] Check if this specific actor, found using his display name, has a position saved. If he has he is moved to that location and than removed from the dict of actor saved
  (bind _player_actor (Class|IGet|GetPlayer&Actor(Message) _returnvalue_2))
  (if (.ReturnValue (Utilities|Map|Find _player_actor (Utilities|GetClass self)))
    (bind _nameposition (Class|IGet|GetNamePosition(Message) (Game|GetGameInstance)))
    (if (.ReturnValue (Utilities|Map|Find _nameposition (Utilities|GetDisplayName self)))
      (Transformation|SetWorldLocation (Variables|Default|GetStaticMesh) (.Value (Utilities|Map|Find _player_actor (Utilities|GetClass self))) false false)
      (Class|IRemove|RemoveActor(Message) _returnvalue_2 _self)
      ;[1 1 1] Check if he is supposed to be attached to the player. If he is, he attach himself to the player and check the variables used to check for attachments
      (bind _isattachedoutput (Class|IControlAttach|IsAttachedOutput(Message) _returnvalue))
      (if _isattachedoutput
        (CallFunction|Attach _self (Game|Player|GetPlayerPawn 0))
        (Class|IControlAttach|IsAttachedInput(Message) _returnvalue true)))))

(fn ConstructionScript)

(fn IsAttachedOutput
  (return (Variables|Default|GetisAttached)))